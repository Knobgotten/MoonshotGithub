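; Moon boss actor that faces the player every Tick and takes damage from ExpOrbProjectile hits.
; Each hit destroys the projectile, plays a sound and hurt animation, and decrements Health.
; When health runs out, a DoOnce-guarded sequence spawns a huge explosion above the moon and hides its mesh.
; After short delays it shows an Error widget and quits the game outright.
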(event EventBeginPlay)

(event Collision|EventActorBeginOverlap
  (params (OtherActor :type Actor%20Object%20Reference)))

(event EventTick
  (params (DeltaSeconds :type Float%20%28single-precision%29))
  (bind _returnvalue (Transformation|GetActorLocation))
  (bind _returnvalue_2 (Game|Player|GetPlayerPawn 0))
  (bind _returnvalue_3 (Transformation|GetActorLocation _returnvalue_2))
  (bind _returnvalue_4 (Math|Rotator|FindLookatRotation _returnvalue _returnvalue_3))
  (Transformation|SetActorRotation (Math|Rotator|MakeRotator (.roll _returnvalue_4) (.pitch _returnvalue_4) (.yaw _returnvalue_4))))

(event Collision|EventHit
  (params (MyComp :type Primitive%20Component%20Object%20Reference) (Other :type Actor%20Object%20Reference) (OtherComp :type Primitive%20Component%20Object%20Reference) (bSelfMoved :type Boolean) (HitLocation :type Vector :default "0, 0, 0") (HitNormal :type Vector :default "0, 0, 0") (NormalImpulse :type Vector :default "0, 0, 0") (Hit :type Hit%20Result%20Structure%20%28by%20ref%29))
  (bind _returnvalue (Transformation|GetActorLocation))
  (Utilities|Casting|CastToExpOrbProjectile Other)
  (Development|PrintString "Hit!")
  (Actor|DestroyActor Other)
  (Audio|PlaySound2D "/Game/Audio/ChipShop_YM_FX_Explo_01_Cue.ChipShop_YM_FX_Explo_01_Cue" 1.0 1.0 0.0 0 0)
  (Components|Animation|PlayAnimation (Variables|SkeletalMeshActor|GetSkeletalMeshComponent) "/Game/Models/Moon/MajoraMoonAnimHurt.MajoraMoonAnimHurt" false)
  (bind _result (Math|Integer|DecrementInt (Variables|Default|GetHealth))
    (:%20%20
      (if (<= _result 0)
        (Utilities|FlowControl|DoOnce false
          (:Completed
            (Effects|SpawnEmitteratLocation "/Game/AdvancedMagicFX13/Particles/P_ky_explosion1.P_ky_explosion1" (Math|Vector|MakeVector (.x _returnvalue) (.y _returnvalue) (+ (.z _returnvalue) 5e+03)) "0, 0, 0" "1000.000000,1000.000000,1000.000000")
            (Audio|PlaySound2D "/Game/Audio/ChipShop_YM_FX_Explo_02.ChipShop_YM_FX_Explo_02" 0.5 1.0 0.0 0 0)
            (Development|SetHiddeninGame (Variables|SkeletalMeshActor|GetSkeletalMeshComponent) true true)
            (Utilities|FlowControl|Delay 2.0)
            (Audio|PlaySound2D "/Game/Audio/ChipShop_YM_FX_Ill.ChipShop_YM_FX_Ill" 1.0 1.0 0.0 0 0)
            (bind _returnvalue_2 (UserInterface|CreateWidget "/Game/Error.Error_C"))
            (UserInterface|Viewport|AddtoViewport _returnvalue_2 0)
            (Utilities|FlowControl|Delay 1.0)
            (Game|QuitGame 0 "Quit" false)))))))

(fn ConstructionScript)