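; PortalrenderEnabler is a trigger actor that switches portal rendering on and off based on player presence.
; When the player pawn begins overlapping it, it sets RenderEnabled on the referenced portal and that portal's TargetPortal.
; When the player pawn stops overlapping, it clears the flag on both, so the linked pair is toggled together without using Tick.
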(event EventBeginPlay)

(event Collision|EventActorBeginOverlap
  (params (OtherActor :type Actor%20Object%20Reference))
  (bind _portalref (Variables|Default|GetPortalRef))
  (if (== OtherActor (Game|Player|GetPlayerPawn 0))
    (Variables|/Game/PortalsBP/Blueprints/PortalBP.PortalBP_C|SetRenderEnabled _portalref true)
    (Variables|/Game/PortalsBP/Blueprints/PortalBP.PortalBP_C|SetRenderEnabled (Variables|/Game/PortalsBP/Blueprints/PortalBP.PortalBP_C|GetTargetPortal _portalref) true)))

(event EventTick
  (params (DeltaSeconds :type Float%20%28single-precision%29)))

(event Collision|EventActorEndOverlap
  (params (OtherActor :type Actor%20Object%20Reference))
  (bind _portalref (Variables|Default|GetPortalRef))
  (if (== OtherActor (Game|Player|GetPlayerPawn 0))
    (Variables|/Game/PortalsBP/Blueprints/PortalBP.PortalBP_C|SetRenderEnabled _portalref false)
    (Variables|/Game/PortalsBP/Blueprints/PortalBP.PortalBP_C|SetRenderEnabled (Variables|/Game/PortalsBP/Blueprints/PortalBP.PortalBP_C|GetTargetPortal _portalref) false)))

(fn ConstructionScript)