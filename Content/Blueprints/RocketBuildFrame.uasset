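; Rocket assembly frame that shows collected rocket parts and sends the game to BossLevel once the rocket is complete.
; ShowPiece matches the piece's class display name by substring to Chair, Thruster, WingL, WingR or Body, then swaps that part's grey component for its colored one and flags it found.
; Every match runs a shared completion check, which plays a sound and loads the level after a short delay when all parts are found.
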(event Custom|ShowPiece
  (params (Piece :type Rocket%20Piece%20Parent%20Class%20Reference))
  (bind _returnvalue (Utilities|GetClassDisplayName Piece))
  (if (Utilities|String|Contains _returnvalue "Chair")
    (Rendering|SetVisibility (Variables|Default|GetChairGrey) false false)
    (Rendering|SetVisibility (Variables|Default|GetChairColored) true false)
    (bind _output_get (Variables|Default|SetChairFound true))
    (if (Math|Boolean|ANDBoolean _output_get (stale _output_get_2) (stale _output_get_3) (stale _output_get_4) (stale _output_get_5)) :!label _label
      (Audio|PlaySound2D "/Game/Audio/ChipShop_YM_Arp_G_m_16.ChipShop_YM_Arp_G_m_16" 1.0 1.0 0.0 0 0)
      (Utilities|FlowControl|Delay 5.0)
      (Game|OpenLevel(byName) "BossLevel"))
    (elif (Utilities|String|Contains _returnvalue "Thruster")
      (Rendering|SetVisibility (Variables|Default|GetThrusterGrey) false false)
      (Rendering|SetVisibility (Variables|Default|GetThrusterColored) true false)
      (bind _output_get_2 (Variables|Default|SetThrusterFound true))
      (goto _label)
      (elif (Utilities|String|Contains _returnvalue "WingL")
        (Rendering|SetVisibility (Variables|Default|GetWingLGrey) false false)
        (Rendering|SetVisibility (Variables|Default|GetWingLColored) true false)
        (bind _output_get_3 (Variables|Default|SetWingLFound true))
        (goto _label)
        (elif (Utilities|String|Contains _returnvalue "WingR")
          (Rendering|SetVisibility (Variables|Default|GetWingRGrey) false false)
          (Rendering|SetVisibility (Variables|Default|GetWingRColored) true false)
          (bind _output_get_4 (Variables|Default|SetWingRFound true))
          (goto _label)
          (elif (Utilities|String|Contains _returnvalue "Body")
            (Rendering|SetVisibility (Variables|Default|GetBodyGrey) false false)
            (Rendering|SetVisibility (Variables|Default|GetBodyColored) true false)
            (bind _output_get_5 (Variables|Default|SetBodyFound true))
            (goto _label)))))))

(event EventBeginPlay)

(event Collision|EventActorBeginOverlap
  (params (OtherActor :type Actor%20Object%20Reference)))

(event EventTick
  (params (DeltaSeconds :type Float%20%28single-precision%29)))

(fn ConstructionScript)