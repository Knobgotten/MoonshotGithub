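; RocketBuildTrigger is a trigger actor that installs rocket pieces into the rocket build frame when they enter its overlap.
; Shortly after BeginPlay it finds and caches the level's RocketBuildFrame.
; On overlap with a RocketPieceParent subclass, it compares the actor's class against its PiecesRefs list.
; A match tells the frame to show that piece class and destroys the overlapping actor.
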(event EventBeginPlay
  (Utilities|FlowControl|Delay 0.2)
  (bind _returnvalue (Actor|GetActorOfClass "/Game/Blueprints/RocketBuildFrame.RocketBuildFrame_C"))
  (Variables|Default|SetRocketBuildFrameRef _returnvalue))

(event Collision|EventActorBeginOverlap
  (params (OtherActor :type Actor%20Object%20Reference))
  (bind _returnvalue (Utilities|GetClass OtherActor))
  (if (Utilities|ClassIsChildOf _returnvalue "/Game/Models/Rocket/RocketPieceParent.RocketPieceParent_C")
    (for _array_element (Variables|Default|GetPiecesRefs)
      (if (== _array_element _returnvalue)
        (Default|ShowPiece (Variables|Default|GetRocketBuildFrameRef) _array_element)
        (Actor|DestroyActor OtherActor)))))

(event EventTick
  (params (DeltaSeconds :type Float%20%28single-precision%29)))

(fn ConstructionScript)