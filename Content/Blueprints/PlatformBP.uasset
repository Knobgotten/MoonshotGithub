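; Platform trigger that overrides planetary gravity while the player stands on it.
; On player overlap it flags the character as on-platform, clears HasGravity and points every GravityCharacter's gravity along the platform's inverted up vector.
; On exit it clears the flag and, after three seconds, reattaches the player to the nearest planet unless they are back on a platform.
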(event EventBeginPlay)

(event Collision|EventActorBeginOverlap
  (params (OtherActor :type Actor%20Object%20Reference))
  (bind _returnvalue (Transformation|GetActorUpVector))
  (bind _returnvalue_2 (* _returnvalue -1.0))
  (Utilities|IsPlayer? OtherActor
    (:True
      (Utilities|SetonPlatform true)
      (bind _asmy_gravity_character (Utilities|Casting|CastToMyGravityCharacter (Game|GetPlayerCharacter 0)))
      (Variables|/DirGravity/Character/BP_GravityCharacter.BP_GravityCharacter_C|SetHasGravity _asmy_gravity_character false)
      (CallFunction|SetGravity _returnvalue_2)
      (Development|PrintString (Utilities|String|Append "GravitySetTo" (Utilities|String|ToString(Vector) _returnvalue_2))))))

(event Collision|EventActorEndOverlap
  (params (OtherActor :type Actor%20Object%20Reference))
  (Utilities|IsPlayer? OtherActor
    (:True
      (Utilities|SetonPlatform false)
      (Utilities|FlowControl|Delay 3.0)
      (bind _asmy_gravity_character (Utilities|Casting|CastToMyGravityCharacter (Game|GetPlayerCharacter 0)))
      (if (not (Variables|/Game/Blueprints/MyGravityCharacter.MyGravityCharacter_C|GetOnPlatform? _asmy_gravity_character))
        (bind _asmy_gravity_character_2 (Utilities|Casting|CastToMyGravityCharacter (Game|GetPlayerCharacter 0)))
        (Default|AttachtoNearestPlanet _asmy_gravity_character_2)
        (Development|PrintString (Utilities|String|Append "GravityOFF" ""))))))

(fn ConstructionScript)

(fn SetGravity
  (params (NewGravityDirection :type Vector))
  (bind _outactors (Actor|GetAllActorsOfClass "/Script/DirGravity.GravityCharacter"))
  (for _array_element _outactors
    (Class|GravityMovementComponent|SetGravityDirection (Class|GravityCharacter|GetGravityMovementComponent _array_element) NewGravityDirection)))